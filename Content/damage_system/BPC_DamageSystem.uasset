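; Actor component that handles damage and core stats: health, mana, XP and player level.
; TakeDamage uses the CanBeDamaged macro to route hits to block, damage or ignore based on death, invincibility and blocking state, with per-hit overrides from DamageInfo.
; It fires OnBlocked, OnDeath, or OnDamageResponse for interruptible or forced-interrupt hits.
; Heal, ManaRegen and KillXP add clamped amounts while alive, and PlayerLevel increments the level.
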(event EventBeginPlay)

(event EventTick
  (params (DeltaSeconds :type Float%20%28single-precision%29)))

(fn Heal
  (params (Amount :type Float%20%28double-precision%29))
  ;[0.2014 1 0.2092] heal functionality
  (if (not (Variables|Default|GetIsDead))
    (bind _output_get (Variables|Default|SetHealth (Math|Float|Clamp(Float) (+ Amount (Variables|Default|GetHealth)) 0.0 (Variables|Default|GetMaxHealth))))
    (return _output_get)))

(fn TakeDamage
  (params (DamageInfo :type S%20Damage%20Info%20Structure))
  (bind (_amount _damagetype _damageresponse _shoulddamageinvincible _canbeblocked _canbeparried _shouldforceinterupt) (Utilities|Struct|BreakS_DamageInfo DamageInfo))
  ;[1 0.1201 0.06042] damage functions
  (Utilities|CanbeDamaged _shoulddamageinvincible _canbeblocked
    (:BlockDamage
      (Default|CallOnBlocked _canbeparried)
      (return false))
    (:DoDamage
      (bind _output_get (Variables|Default|SetHealth (- (Variables|Default|GetHealth) _amount)))
      (if (<= _output_get 0.0)
        (Variables|Default|SetIsDead true)
        (Default|CallOnDeath)
        (return true)
        (elif (or (Variables|Default|GetIsInterruptible) _shouldforceinterupt)
          (Default|CallOnDamageResponse _damageresponse)
          (return true))))
    (:NoDamage
      (return false))))

(fn ManaRegen
  (params (Amount :type Float%20%28double-precision%29))
  (if (not (Variables|Default|GetIsDead))
    (bind _output_get (Variables|Default|SetMana (Math|Float|Clamp(Float) (+ Amount (Variables|Default|GetMana)) 0.0 (Variables|Default|GetMaxMana))))
    (return _output_get)))

(fn KillXP
  (params (Amount :type Float%20%28double-precision%29))
  (if (not (Variables|Default|GetIsDead))
    (bind _output_get (Variables|Default|SetXP (Math|Float|Clamp(Float) (+ Amount (Variables|Default|GetXP)) 0.0 (Variables|Default|GetMaxXP))))
    (return _output_get)))

(fn PlayerLevel
  (if true
    (bind _playerlevel (CallFunction|PlayerLevel))
    (bind _output_get (Variables|Default|SetPlayerLevel (+ _playerlevel 1.0)))
    (return _output_get)))