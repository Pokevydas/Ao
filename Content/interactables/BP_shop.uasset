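; BP_shop is an interactable shop that reports a "Talk" prompt with zero hold duration and manages the shop's UI.
; Interact opens the Shop_interact widget, switches input to UI-only with a visible cursor, and sets InInteract.
; That flag gates Shop_talk and Shopbutton, which add the dialogue and shop menu widgets respectively.
; Exit removes all three widgets and restores game-only input, leaving InInteract and the cursor setting unchanged.
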(event Custom|Shop%20button
  (bind _shopinteractref (Variables|Default|GetShopInteractref))
  (if (Variables|Default|GetinInteract)
    (|SetBy-RefVar _shopinteractref _shopinteractref)
    (bind _returnvalue (UserInterface|CreateWidget "/Game/UI/interactions/Shop_menu.Shop_menu_C" (Game|GetPlayerController 0)))
    (bind _output_get (Variables|Default|SetShopMenuref _returnvalue))
    (UserInterface|Viewport|AddtoViewport _output_get 0)
    (Variables|/Script/Engine.PlayerController|SetbShowMouseCursor (Game|GetPlayerController 0) true)))

(event Custom|Shop_talk
  (bind _shopinteractref (Variables|Default|GetShopInteractref))
  (if (Variables|Default|GetinInteract)
    (|SetBy-RefVar _shopinteractref _shopinteractref)
    (bind _returnvalue (UserInterface|CreateWidget "/Game/UI/interactions/Shop_talk.Shop_talk_C" (Game|GetPlayerController 0)))
    (bind _output_get (Variables|Default|SetShopTalkref _returnvalue))
    (UserInterface|Viewport|AddtoViewport _output_get 0)
    (Variables|/Script/Engine.PlayerController|SetbShowMouseCursor (Game|GetPlayerController 0) true)))

(event Custom|Exit
  (Widget|RemovefromParent (Variables|Default|GetShopMenuref))
  (Input|SetInputModeGameOnly (Game|GetPlayerController 0) false))

(event EventInteract
  (params (Interactor :type Actor%20Object%20Reference))
  (bind _returnvalue (UserInterface|CreateWidget "/Game/UI/interactions/Shop_interact.Shop_interact_C" (Game|GetPlayerController 0)))
  (bind _output_get (Variables|Default|SetShopInteractref _returnvalue))
  (UserInterface|Viewport|AddtoViewport _output_get 0)
  (Input|SetInputModeUIOnly (Game|GetPlayerController 0) 0 "DoNotLock" false)
  (Variables|/Script/Engine.PlayerController|SetbShowMouseCursor (Game|GetPlayerController 0) true)
  (Variables|Default|SetinInteract true))

(fn ConstructionScript)

(fn GetHoldDuration
  (return 0.0))

(fn GetInteraction
  (return "Talk"))

(fn GetInteractionType
  (return "NewEnumerator0"))