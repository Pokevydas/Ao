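; BP_spawnPoint is an interactable spawn point that is activated on first use.
; Interact calls Activate while inactive, which sets IsActivated and plays a timeline that rotates and moves the MagicCircle.
; Later interactions call OpenMenu, which currently only sets the same flag.
; Interaction getters supply the hold duration and switch the prompt and interaction type based on activation state.
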(event Custom|activate
  (bind _magic_circle (Variables|Default|Getmagic%20circle))
  (Variables|Default|SetIsActivated true)
  (bind (_direction _rotation _height) (Timeline|Timeline Play)
    (:Update
      (Transformation|SetRelativeRotation _magic_circle (Math|Rotator|MakeRotator 0.0 0.0 _rotation) false false)
      (Transformation|SetRelativeLocation _magic_circle (Math|Vector|MakeVector 0.0 _height 0.0) false false))))

(event Custom|open%20menu
  (Variables|Default|SetIsActivated true))

(event EventInteract
  (params (Interactor :type Actor%20Object%20Reference))
  (if (Variables|Default|GetIsActivated)
    (CallFunction|OpenMenu)
    (else
      (CallFunction|Activate))))

(fn ConstructionScript)

(fn GetHoldDuration
  (return (Variables|Default|GetHoldDuration)))

(fn GetInteraction
  (return (select (Variables|Default|GetIsActivated) "Interact" "Activate")))

(fn GetInteractionType
  (if (Variables|Default|GetIsActivated)
    (return "NewEnumerator0")
    (else
      (return "NewEnumerator1"))))