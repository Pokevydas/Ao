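; BP_slime is a slime interactable Blueprint that is currently a stub with no gameplay behavior.
; It exposes an Interact event plus health, mana, XP, level, healing and damage functions, which appear to come from shared interfaces.
; Interact is empty, every stat function returns zero, TakeDamage always returns false, and two health getter calls sit unconnected in the event graph.
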(event EventInteract
  (params (Interactor :type Actor%20Object%20Reference)))

(fn ConstructionScript)

(fn GetCurrentHealth
  (return 0.0))

(fn GetCurrentMana
  (return 0.0))

(fn GetCurrentXP
  (return 0.0))

(fn GetMaxHealth
  (return 0.0))

(fn GetMaxMana
  (return 0.0))

(fn GetMaxXP
  (return 0.0))

(fn Heal
  (params (Amount :type Float%20%28double-precision%29))
  (return 0.0))

(fn KillXP
  (params (Amount :type Float%20%28double-precision%29))
  (return 0.0))

(fn ManaRegen
  (params (Amount :type Float%20%28double-precision%29))
  (return 0.0))

(fn PlayerLevel
  (return 0.0))

(fn TakeDamage
  (params (DamageInfo :type S%20Damage%20Info%20Structure))
  (return false))