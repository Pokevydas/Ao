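; An interactable item pickup actor that a player can pick up.
; It supplies the interaction interface with a "Pick up" prompt, a fixed interaction type and a zero hold duration.
; On Interact it prints a message naming the item and interactor, plays a sound at its location and destroys itself, without storing anything in an inventory.
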(event EventInteract
  (params (Interactor :type Actor%20Object%20Reference))
  (Development|PrintString (Utilities|String|ToString(Text) (Utilities|Text|FormatText "Added {item name} to the inventory of {actor name} " (Utilities|GetDisplayName self) (Utilities|GetDisplayName Interactor))))
  (Audio|PlaySoundatLocation 0 (Transformation|GetActorLocation) "0, 0, 0" 1.0 1.0 0.0 0 0 0 0)
  (Actor|DestroyActor))

(fn ConstructionScript)

(fn GetHoldDuration
  (return 0.0))

(fn GetInteraction
  (return "Pick up"))

(fn GetInteractionType
  (return "NewEnumerator0"))