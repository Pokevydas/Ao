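; Interactable spawn point that acts as a teleport pad with activated and inactive states.
; Interact loads ThirdPersonLevel through OpenMenu when activated, otherwise Activate sets the flag and loops teleport animations on three nested circle components.
; Interaction getters supply a hold duration, plus a prompt and type that follow the state.
; BeginPlay already sets it activated, so the activation branch is skipped by default.
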(event Custom|activate
  (Variables|Default|SetIsActivated true)
  (Components|Animation|PlayAnimation (Variables|Default|Getcircle) "/Game/interactables/circle/teleport.teleport" true)
  (Components|Animation|PlayAnimation (Variables|Default|Getinner_circle) "/Game/interactables/circle/teleport1.teleport1" true)
  (Components|Animation|PlayAnimation (Variables|Default|GetInner_inner_circle) "/Game/interactables/circle/teleport12.teleport12" true))

(event Custom|open%20menu
  (Variables|Default|SetIsActivated true)
  (Game|OpenLevel(byName) "ThirdPersonLevel"))

(event EventBeginPlay
  (Variables|Default|SetIsActivated true))

(event EventInteract
  (params (Interactor :type Actor%20Object%20Reference))
  (if (Variables|Default|GetIsActivated)
    (CallFunction|OpenMenu)
    (else
      (CallFunction|Activate))))

(fn ConstructionScript)

(fn GetHoldDuration
  (return (Variables|Default|GetHoldDuration)))

(fn GetInteraction
  (return (select (Variables|Default|GetIsActivated) "Interact" "Activate")))

(fn GetInteractionType
  (if (Variables|Default|GetIsActivated)
    (return "NewEnumerator0")
    (else
      (return "NewEnumerator1"))))