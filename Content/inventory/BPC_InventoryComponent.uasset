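; Inventory component that stores picked-up items in a fixed-size array of item structs and shows them in a W_InventoryGrid widget.
; AddToInventory walks the slots in order, stacking a matching stackable item up to a per-item cap or inserting at an empty slot, whichever comes first.
; A successful add refreshes the grid and destroys the item actor.
; The inventory input action opens the grid with a mouse cursor and UI-only input.
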(event Input|EnhancedActionEvents|EnhancedInputActionIA_inventory
  (params (ActionValue :type Boolean) (ElapsedSeconds :type Float%20%28double-precision%29) (TriggeredSeconds :type Float%20%28double-precision%29) (InputAction :type Input%20Action%20Object%20Reference :default "/Game/ThirdPerson/Input/Actions/IA_inventory.IA_inventory"))
  (bind _returnvalue (Game|GetPlayerController 0))
  (bind _inventoryref (Variables|Default|GetInventoryRef))
  (bind _inventoryref_2 (Variables|Default|GetInventoryRef))
  (:Triggered
    (if (not (UserInterface|Viewport|IsinViewport _inventoryref))
      (UserInterface|Viewport|AddtoViewport _inventoryref 0)
      (Variables|/Script/Engine.PlayerController|SetbShowMouseCursor _returnvalue true)
      (Input|SetInputModeUIOnly _returnvalue _inventoryref_2 "DoNotLock" false)
      (Variables|/Script/UMG.UserWidget|SetbIsFocusable _inventoryref_2 true))))

(event EventBeginPlay
  (bind _returnvalue (UserInterface|CreateWidget "/Game/inventory/W_InventoryGrid.W_InventoryGrid_C"))
  (Variables|Default|SetInventoryRef _returnvalue)
  (Utilities|Array|Resize (Variables|Default|GetItems) (Variables|Default|GetInventorySize))
  (Default|RefreshInventory (Variables|Default|GetInventoryRef) self))

(fn AddtoInventory
  (params (Actor :type BP%20Base%20Item%20Object%20Reference))
  (bind _items (Variables|Default|GetItems))
  (LocalVariables|SetL%20Item%20Interacted Actor)
  (for (_array_element _array_index) (Variables|Default|GetItems)
    (Utilities|IsValid Actor
      (:Is%20Valid
        (Variables|Default|SetCurrentIndex _array_index)
        (bind (_can_add_ _new_item_amount) (CallFunction|ShouldStackItems? _array_element (Variables|/Game/inventory/BP_baseItem.BP_baseItem_C|GetItem (LocalVariables|GetL%20Item%20Interacted))))
        (if _can_add_
          (Variables|Default|SetNewItemAmount _new_item_amount)
          (Utilities|Array|SetArrayElem (Variables|Default|GetItems) (Variables|Default|GetCurrentIndex) (Utilities|Struct|MakeS_item (.ItemInventory? (Utilities|Struct|BreakS_item (Variables|/Game/inventory/BP_baseItem.BP_baseItem_C|GetItem (LocalVariables|GetL%20Item%20Interacted)))) (.ItemName (Utilities|Struct|BreakS_item (Variables|/Game/inventory/BP_baseItem.BP_baseItem_C|GetItem (LocalVariables|GetL%20Item%20Interacted)))) (.Itemdescription (Utilities|Struct|BreakS_item (Variables|/Game/inventory/BP_baseItem.BP_baseItem_C|GetItem (LocalVariables|GetL%20Item%20Interacted)))) (.Stackable? (Utilities|Struct|BreakS_item (Variables|/Game/inventory/BP_baseItem.BP_baseItem_C|GetItem (LocalVariables|GetL%20Item%20Interacted)))) (Variables|Default|GetNewItemAmount) (.ItemMesh (Utilities|Struct|BreakS_item (Variables|/Game/inventory/BP_baseItem.BP_baseItem_C|GetItem (LocalVariables|GetL%20Item%20Interacted)))) (.ItemImage (Utilities|Struct|BreakS_item (Variables|/Game/inventory/BP_baseItem.BP_baseItem_C|GetItem (LocalVariables|GetL%20Item%20Interacted)))) (.IsHealable (Utilities|Struct|BreakS_item (Variables|/Game/inventory/BP_baseItem.BP_baseItem_C|GetItem (LocalVariables|GetL%20Item%20Interacted)))) (.ItemHealAmount (Utilities|Struct|BreakS_item (Variables|/Game/inventory/BP_baseItem.BP_baseItem_C|GetItem (LocalVariables|GetL%20Item%20Interacted))))))
          (Default|RefreshInventory (Variables|Default|GetInventoryRef) self :!label _label)
          (Actor|DestroyActor (LocalVariables|GetL%20Item%20Interacted))
          (return)
          (else
            (bind _has_space (CallFunction|SpaceinInventory? _new_item_amount))
            (if _has_space
              (Utilities|Array|Insert _items (Variables|/Game/inventory/BP_baseItem.BP_baseItem_C|GetItem (LocalVariables|GetL%20Item%20Interacted)) (Variables|Default|GetCurrentIndex))
              (Utilities|Array|RemoveIndex _items (- (Variables|Default|GetInventorySize) (Variables|Default|GetCurrentIndex)))
              (goto _label))))))))

(fn ShouldStackItems?
  (params (Item%20from%20Inventory :type S%20Item%20Structure) (Item%20from%20current%20actor :type S%20Item%20Structure))
  (bind (_iteminventory_ _itemname _itemdescription _stackable_ _itemamount) (Utilities|Struct|BreakS_item Item%20from%20Inventory))
  (bind (_iteminventory__2 _itemname_2 _itemdescription_2 _stackable__2 _itemamount_2) (Utilities|Struct|BreakS_item Item%20from%20current%20actor))
  (bind _returnvalue (+ _itemamount _itemamount_2))
  (if (Math|Boolean|ANDBoolean _iteminventory__2 (Utilities|Enum|Equal(Enum) _itemname _itemname_2) _stackable__2 (<= _returnvalue (Variables|Default|GetMaxAmountPerItem)))
    (return true _returnvalue)
    (else
      (return false _itemamount))))

(fn SpaceinInventory?
  (params (Item%20Amount%20From%20Inventory :type Integer))
  (if (== Item%20Amount%20From%20Inventory 0)
    (return true)
    (else
      (return false))))